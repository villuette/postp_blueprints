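; Floating enemy health display actor that shows an enemyStatsView widget through its View component.
; Each tick it rotates its root from the widget's location toward the player camera, billboard-style.
; BindInitialStats stores the initial health and fills the health bar.
; UpdateStats sets the bar to current HP over initial health and prints that ratio to screen.
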(event EventBeginPlay)

(event Collision|EventActorBeginOverlap
  (params (OtherActor :type Actor%20Object%20Reference)))

(event EventTick
  (params (DeltaSeconds :type Float%20%28single-precision%29))
  (Transformation|SetWorldRotation (Variables|Default|GetDefaultSceneRoot) (Math|Rotator|FindLookatRotation (Transformation|GetWorldLocation (Variables|Default|Getview)) (Transformation|GetWorldLocation (Variables|/Script/Engine.PlayerCameraManager|GetTransformComponent (Game|GetPlayerCameraManager 0)))) false false))

(fn ConstructionScript)

(fn UpdateStats
  (params (current_HP :type Integer))
  (bind _returnvalue (Math|Conversions|ToFloat(Integer) current_HP))
  (bind _inithealth (Variables|Default|GetinitHealth))
  (bind _returnvalue_2 (Math|Conversions|ToFloat(Integer) _inithealth))
  (bind _returnvalue_3 (/ _returnvalue _returnvalue_2))
  (bind _asenemy_stats_view (Utilities|Casting|CastToenemyStatsView (UserInterface|GetWidget (Variables|Default|Getview))))
  (Progress|SetPercent (Variables|/Game/blueprints/core/enemyStatsView.enemyStatsView_C|Gethealthbar _asenemy_stats_view) _returnvalue_3)
  (Development|PrintString (Utilities|String|ToString(Float) _returnvalue_3)))

(fn BindInitialStats
  (params (initHealth :type Integer))
  (Variables|Default|SetinitHealth initHealth)
  (bind _asenemy_stats_view (Utilities|Casting|CastToenemyStatsView (UserInterface|GetWidget (Variables|Default|Getview))))
  (Progress|SetPercent (Variables|/Game/blueprints/core/enemyStatsView.enemyStatsView_C|Gethealthbar _asenemy_stats_view) 1.0))