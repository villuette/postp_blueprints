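; Weapon actor that fires projectiles and tracks loaded and reserve (AverageAmmo) ammunition.
; Shoot spends a round and spawns a damage-bound projectile at the gun tip, leaving Direction unused, while UpdateAmmoInHUD writes reserve/loaded counts.
; Reload refills from reserve, but its partial branch zeroes the reserve before computing the load, so adds no rounds.
; Hit only casts to MainPlayer; the inventory pickup call is disconnected.
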(event EventBeginPlay)

(event Collision|EventActorBeginOverlap
  (params (OtherActor :type Actor%20Object%20Reference)))

(event EventTick
  (params (DeltaSeconds :type Float%20%28single-precision%29)))

(event Collision|EventHit
  (params (MyComp :type Primitive%20Component%20Object%20Reference) (Other :type Actor%20Object%20Reference) (OtherComp :type Primitive%20Component%20Object%20Reference) (bSelfMoved :type Boolean) (HitLocation :type Vector :default "0, 0, 0") (HitNormal :type Vector :default "0, 0, 0") (NormalImpulse :type Vector :default "0, 0, 0") (Hit :type Hit%20Result%20Structure%20%28by%20ref%29))
  (bind _asmain_player (Utilities|Casting|CastToMainPlayer Other)))

(fn ConstructionScript)

(fn Shoot
  (params (gun_tip :type Transform) (direction :type Vector))
  (if (> (Variables|Default|Getammo_loaded) 0)
    (bind _result (Math|Integer|DecrementInt (Variables|Default|Getammo_loaded))
      (:%20%20
        (Variables|Default|Setammo_loaded _result)
        (bind _returnvalue (Game|SpawnActorfromClass "/Game/blueprints/core/Projectile.Projectile_C" gun_tip "AdjustIfPossibleButAlwaysSpawn" 0 0))
        (Default|BindDamages _returnvalue 2e+01 0.0)))
    (else
      (Development|PrintString "Relload needed!"))))

(fn UpdateAmmoinHUD
  (params (hud :type Player%20Ui%20Object%20Reference))
  (Rendering|Components|TextRender|SetText (Variables|/Game/ui/player_ui.player_ui_C|GetAmmo_value_hud hud) (Utilities|Text|ToText(String) (Utilities|String|Append (Utilities|String|ToString(Integer) (Variables|Default|Getaverage_ammo)) "/" (Utilities|String|ToString(Integer) (Variables|Default|Getammo_loaded))))))

(fn Reload
  (if (> (Variables|Default|Getaverage_ammo) 0)
    (Development|PrintString "Reloading...")
    (if (> (- (Variables|Default|Getaverage_ammo) (- (Variables|Default|Getmax_loaded) (Variables|Default|Getammo_loaded))) 0)
      (Variables|Default|Setaverage_ammo (- (Variables|Default|Getaverage_ammo) (- (Variables|Default|Getmax_loaded) (Variables|Default|Getammo_loaded))))
      (Variables|Default|Setammo_loaded (Variables|Default|Getmax_loaded))
      (else
        (Variables|Default|Setaverage_ammo 0)
        (Variables|Default|Setammo_loaded (+ (- (Variables|Default|Getaverage_ammo) (- (Variables|Default|Getmax_loaded) (Variables|Default|Getammo_loaded))) (Variables|Default|Getmax_loaded)))))
    (else
      (Development|PrintString "out of ammo"))))