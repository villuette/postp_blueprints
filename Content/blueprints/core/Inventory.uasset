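; Inventory Blueprint that stores picked-up weapons and tracks the current one.
; PickUpWeapon adds the weapon to the list, copies its static mesh onto the supplied arm component, then disables the weapon mesh's collision, hides the actor and sets it as current.
; A bound widget reference receives a visibility toggle call from ToggleInventory, which also prints a debug string.
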(event EventBeginPlay)

(event EventTick
  (params (DeltaSeconds :type Float%20%28single-precision%29)))

(fn PickUpWeapon
  (params (Weapon :type Weapon%20Object%20Reference) (Arm :type Static%20Mesh%20Component%20Object%20Reference))
  (bind _returnvalue (Actor|GetComponentbyClass Weapon "/Script/Engine.StaticMeshComponent"))
  (Utilities|Array|Add (Variables|Default|GetWeapons) Weapon)
  (Components|StaticMesh|SetStaticMesh Arm (Variables|/Script/Engine.StaticMeshComponent|GetStaticMesh _returnvalue))
  (Collision|SetCollisionEnabled _returnvalue "NoCollision")
  (Rendering|SetActorHiddenInGame Weapon true)
  (Variables|Default|SetCurrentWeapon Weapon))

(fn BindWidget
  (params (Widget :type Widget%20Component%20Object%20Reference))
  (Variables|Default|Setwidget Widget))

(fn ToggleInventory
  (Development|PrintString "TOGGLED")
  (Rendering|ToggleVisibility (Variables|Default|Getwidget) false))