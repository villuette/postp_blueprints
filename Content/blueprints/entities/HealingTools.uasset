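; HealingTools is a pickup actor that changes the player's health when applied.
; ApplyPick adds a fixed amount to CurrentHealth and takes the result modulo MaxHealth, so health wraps around at the maximum instead of clamping.
; It then refreshes the player's HUD, prints a debug message and destroys itself.
; The construction script only calls its parent, and the event graph holds no logic.
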(event EventBeginPlay)

(event Collision|EventActorBeginOverlap
  (params (OtherActor :type Actor%20Object%20Reference)))

(event EventTick
  (params (DeltaSeconds :type Float%20%28single-precision%29)))

(fn ConstructionScript
  (|CallParentFunction))

(fn ApplyPick
  (params (player :type Main%20Player%20Object%20Reference))
  (Variables|/Game/blueprints/entities/MainPlayer.MainPlayer_C|SetcurrentHealth player (Math|Integer|%(Integer) (+ (Variables|/Game/blueprints/entities/MainPlayer.MainPlayer_C|GetcurrentHealth player) 20) (Variables|/Game/blueprints/entities/MainPlayer.MainPlayer_C|GetmaxHealth player)))
  (Default|UpdateHUD (Variables|/Game/blueprints/entities/MainPlayer.MainPlayer_C|Getplayer_hud_object player) player)
  (Development|PrintString "Healed")
  (Actor|DestroyActor))