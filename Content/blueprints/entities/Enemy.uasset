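; Enemy actor that takes resistance-scaled physical and magical damage from projectiles and destroys itself at zero health.
; On begin play it binds its initial health to a stats view child actor.
; Projectile hits call TakeDamage, then destroy the projectile.
; TakeDamage truncates each reduced damage type, updates the stats view with the new health and calls Die when health runs out.
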(event EventBeginPlay
  (bind _inithealth (Variables|Default|GetinitHealth))
  (bind _asenemy_stats_view_actor (Utilities|Casting|CastToenemyStatsViewActor (Variables|/Script/Engine.ChildActorComponent|GetChildActor (Variables|Default|GetstatsView))))
  (Default|BindInitialStats _asenemy_stats_view_actor _inithealth)
  (Variables|Default|SetHealth _inithealth))

(event EventTick
  (params (DeltaSeconds :type Float%20%28single-precision%29)))

(event Collision|EventHit
  (params (MyComp :type Primitive%20Component%20Object%20Reference) (Other :type Actor%20Object%20Reference) (OtherComp :type Primitive%20Component%20Object%20Reference) (bSelfMoved :type Boolean) (HitLocation :type Vector :default "0, 0, 0") (HitNormal :type Vector :default "0, 0, 0") (NormalImpulse :type Vector :default "0, 0, 0") (Hit :type Hit%20Result%20Structure%20%28by%20ref%29))
  (bind _asprojectile (Utilities|Casting|CastToProjectile Other))
  (Development|PrintString "damaged")
  (CallFunction|TakeDamage (Variables|/Game/blueprints/core/Projectile.Projectile_C|GetPhysicalDamage _asprojectile) (Variables|/Game/blueprints/core/Projectile.Projectile_C|GetMagicalDamage _asprojectile))
  (Actor|DestroyActor _asprojectile))

(fn ConstructionScript)

(fn TakeDamage
  (params (phys :type Float%20%28single-precision%29) (mag :type Float%20%28single-precision%29))
  (bind _output_get (Variables|Default|SetHealth (- (Variables|Default|GetHealth) (Math|Float|Truncate (* (- 1.0 (Variables|Default|GetPhysResistance)) phys)))))
  (bind _output_get_2 (Variables|Default|SetHealth (- _output_get (Math|Float|Truncate (* mag (- 1.0 (Variables|Default|GetMagResistance)))))))
  (Development|PrintString (Utilities|String|Append "Health: " (Utilities|String|ToString(Integer) _output_get_2) "\\nInit Health: " (Utilities|String|ToString(Integer) (Variables|Default|GetinitHealth))))
  (bind _asenemy_stats_view_actor (Utilities|Casting|CastToenemyStatsViewActor (Variables|/Script/Engine.ChildActorComponent|GetChildActor (Variables|Default|GetstatsView)))
    (:then
      (Default|UpdateStats _asenemy_stats_view_actor _output_get_2))
    (:CastFailed
      _))
  (if (<= _output_get_2 0)
    (CallFunction|Die)))

(fn Die
  (Actor|DestroyActor))