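; A pickable world object that adds itself to the player's inventory when the player hits it.
; On BeginPlay it creates an InventoryItem widget from its Name and keeps it as its Item.
; The first hit by a MainPlayer notifies that player, marks the object picked and adds the Item to the player's inventory.
; ApplyPick is a placeholder that only prints a message and is not called here.
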(event EventBeginPlay
  (bind _returnvalue (UserInterface|CreateWidget "/Game/blueprints/core/InventoryItem.InventoryItem_C" 0 (Variables|Default|GetName)))
  (Variables|Default|SetItem _returnvalue))

(event Collision|EventHit
  (params (MyComp :type Primitive%20Component%20Object%20Reference) (Other :type Actor%20Object%20Reference) (OtherComp :type Primitive%20Component%20Object%20Reference) (bSelfMoved :type Boolean) (HitLocation :type Vector :default "0, 0, 0") (HitNormal :type Vector :default "0, 0, 0") (NormalImpulse :type Vector :default "0, 0, 0") (Hit :type Hit%20Result%20Structure%20%28by%20ref%29))
  (if (not (Variables|Default|Get%20Picked))
    (bind _asmain_player (Utilities|Casting|CastToMainPlayer Other))
    (Default|OnPickObject _asmain_player self)
    (Variables|Default|Set%20Picked true)
    (Development|PrintString "hit player") ; need external modifications for physics simulated object
    (Default|AddItem (Variables|/Game/blueprints/entities/MainPlayer.MainPlayer_C|GetAs%20Player%20Inventory _asmain_player) (Variables|Default|GetItem))))

(fn ConstructionScript)

(fn ApplyPick
  (params (player :type Main%20Player%20Object%20Reference))
  (Development|PrintString "CHANGES ON PICK"))